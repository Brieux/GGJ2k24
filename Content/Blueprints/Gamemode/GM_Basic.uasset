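; GM_Basic is a game mode that runs a timed scoring round.
; On BeginPlay it plays an intro level sequence, waits for its length, then starts a looping timer that counts Timer down.
; AddScore awards points for hits and larger bonuses for PostIted events.
; When the countdown reaches zero it resets the timer, pauses the game and pushes an end-level CommonUI widget through the master controller's stack.
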(event `self.ReceiveBeginPlay`
  (bind _level_sequence (`self.Level Sequence`))
  (bind _outactor (`LevelSequencePlayer.CreateLevelSequencePlayer` _level_sequence))
  (`MovieSceneSequencePlayer.Play` (`LevelSequenceActor.SequencePlayer` _outactor))
  (bind _returnvalue (`MovieSceneSequenceExtensions.GetPlaybackEndSeconds` _level_sequence))
  (`KismetSystemLibrary.Delay` _returnvalue)
  (`self.StartTimer`))

(event `AddScore`
  (params (Hit :type Boolean) (PostIted :type Boolean))
  (if Hit
    (set `self.Score` (+ (`self.Score`) 25.0)))
  (if PostIted
    (set `self.Score` (+ (`self.Score`) 100.0))))

(event `ResetScore`
  (set `self.Score` 0.0))

(event `ResetTimer`
  (`KismetSystemLibrary.K2_ClearAndInvalidateTimerHandle` (`self.TimerHandlerTimer`))
  (set `self.Timer` 600.0))

(event `StartTimer`
  (bind _returnvalue (`KismetSystemLibrary.K2_SetTimerDelegate` (delegate `TimerPlayed`) (`self.Time`) true))
  (set `self.TimerHandlerTimer` _returnvalue))

(event `TimerPlayed`
  (bind _output_get (set `self.Timer` (`KismetMathLibrary.FClamp` (- (`self.Timer`) (`self.Time`)) 0.0 (`self.Timer`))))
  (if (== _output_get 0.0)
    (`self.ResetTimer`)
    (`self.EndOfGame`)))

(event `EndOfGame`
  (`GameplayStatics.SetGamePaused` true)
  (bind _asbp_master_controller (cast `/Game/Blueprints/Controller/BP_MasterController` (`GameplayStatics.GetPlayerController` 0)))
  (`/Game/Blueprints/UI/CUI_StackWidget.PushToStack` (`/Game/Blueprints/Controller/BP_MasterController.StackWidget` _asbp_master_controller) "NewEnumerator1" "/Game/Blueprints/UI/PlayerInterface/CUI_EndLevel.CUI_EndLevel_C"))

(fn `UserConstructionScript`)
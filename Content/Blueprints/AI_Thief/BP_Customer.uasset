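; Shop customer character that browses, leaves or checks out, flees when frightened, takes punches and can be grabbed.
; A random timer or chance roll ends browsing, setting the AI_Customer blackboard behaviour and running an EQS query for a checkout location.
; Buyers restart AI logic with a different nav agent radius.
; Grab switches the mesh to lightweight physics and Ungrab launches it, while punches drain PV toward an empty Die event.
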(event `self.ReceiveBeginPlay`
  (`KismetSystemLibrary.DelayUntilNextTick`)
  (bind _returnvalue (`GameplayStatics.GetActorOfClass` "/Game/Blueprints/AI_Thief/BP_POIManager.BP_POIManager_C"))
  (set `self.AllPointsOfInterest` (`/Game/Blueprints/AI_Thief/BP_POIManager.POIs` _returnvalue)))

(event `BeginNavigationInShop`
  (bind _returnvalue (`KismetSystemLibrary.K2_SetTimerDelegate` (delegate `ItsTimeToGo`) (`KismetMathLibrary.RandomFloatInRange` 100.0 200.0)))
  (set `self.HandlerGetOut` _returnvalue)
  (bind _asai_customer (cast `/Game/Blueprints/AI_Thief/AI_Customer` (`self.GetController`)))
  (`BlackboardComponent.SetValueAsVector` (`AIController.Blackboard` _asai_customer) (`KismetStringLibrary.Conv_StringToName` "GetOut") (`self.K2_GetActorLocation`))
  (set `self.PV` (`self.PV Max`)))

(event `ItsTimeToGo`
  (set `self.DecideToGetAway?` true))

(event `DecideToGoAwy`
  (if (or (`KismetMathLibrary.RandomBoolWithWeight` 0.2) (`self.DecideToGetAway?`))
    (`KismetSystemLibrary.K2_ClearAndInvalidateTimerHandle` (`self.HandlerGetOut`))
    (bind _asai_customer (cast `/Game/Blueprints/AI_Thief/AI_Customer` (`self.GetController`)))
    (`BlackboardComponent.SetValueAsEnum` (`AIController.Blackboard` _asai_customer) (`KismetStringLibrary.Conv_StringToName` "Behaviour") (select `bool` (`self.BuySomething `) :`false` 2 :`true` 1 :!type "Byte"))
    (`self.SwitchType` (`self.BuySomething `))
    (bind _returnvalue (`EnvQueryManager.RunEQSQuery` "/Game/Blueprints/AI_Thief/EQS_Checkout.EQS_Checkout" self "RandomBest5Pct"))
    (add `EnvQueryInstanceBlueprintWrapper.OnQueryFinishedEvent` _returnvalue (delegate `OnQueryFinishedEvent_Event`))
    (else
      (set `self.hasBegunTask` false))))

(event `OnQueryFinishedEvent_Event`
  (params (QueryInstance :type "EnvQueryInstanceBlueprintWrapper Object Reference") (QueryStatus :type "EEnvQueryStatus Enum" :default "Processing"))
  (bind _resultlocations (`EnvQueryInstanceBlueprintWrapper.GetQueryResultsAsLocations` QueryInstance))
  (`BlackboardComponent.SetValueAsVector` (`AIController.Blackboard` (stale `DecideToGoAwy` _asai_customer)) (`KismetStringLibrary.Conv_StringToName` "CheckoutLocation") (`NavigationSystemV1.K2_GetRandomReachablePointInRadius` (`KismetArrayLibrary.Array_Random` _resultlocations) 10.0 null null))
  (set `self.hasBegunTask` false)
  (remove `EnvQueryInstanceBlueprintWrapper.OnQueryFinishedEvent` QueryInstance (delegate `OnQueryFinishedEvent_Event`)))

(event `GetAfraid`
  (set `CharacterMovementComponent.MaxWalkSpeed` 800.0 (`self.CharacterMovement`))
  (bind _asai_customer (cast `/Game/Blueprints/AI_Thief/AI_Customer` (`self.GetController`)))
  (`BlackboardComponent.SetValueAsEnum` (`AIController.Blackboard` _asai_customer) (`KismetStringLibrary.Conv_StringToName` "Behaviour") 3))

(event `ReceivePunch`
  (params (HitLocation :type "Vector Structure"))
  (bind _output_get (set `self.PV` (`KismetMathLibrary.Clamp` (- (`self.PV`) 1) 0 (`self.PV Max`))))
  (if (<= _output_get 0)
    (`self.Die`)))

(event `/Game/Blueprints/FunctionLibrary/BPI_Interaction.Ungrab`
  (params (Direction :type "Vector Structure"))
  (`SkeletalMeshComponent.AddImpulseToAllBodiesBelow` (`self.Mesh`) Direction "None" true true))

(event `Die`)

(fn `Grab`
  (params (PhysicsComp :type "PhysicsConstraintComponent Object Reference"))
  (returns (GrabbedComponent :type "PrimitiveComponent Object Reference"))
  (bind _mesh (`self.Mesh`))
  (`PrimitiveComponent.SetSimulatePhysics` _mesh true)
  (`PrimitiveComponent.SetMassOverrideInKg` _mesh "None" 1.0 true)
  (`PrimitiveComponent.SetCollisionEnabled` (`self.CapsuleComponent`) "NoCollision")
  (`PrimitiveComponent.SetCollisionResponseToChannel` (`self.Mesh`) "ECC_PhysicsBody" "ECR_Ignore")
  (return (`self.Mesh`)))

(fn `SwitchType`
  (params (IsBuyer :type Boolean))
  (if IsBuyer
    (bind _asai_customer (cast `/Game/Blueprints/AI_Thief/AI_Customer` (`self.GetController`)))
    (bind _braincomponent (`AIController.BrainComponent` _asai_customer))
    (`BrainComponent.StopLogic` _braincomponent "")
    (set `NavMovementComponent.NavAgentProps` (make `NavAgentProperties` (select `bool` IsBuyer :`false` 40.0 :`true` 34.0 :!type "Float (single-precision)")) (`self.CharacterMovement`))
    (`BrainComponent.RestartLogic` _braincomponent)))

(fn `UserConstructionScript`)
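; BP_Generation assigns generation IDs to every BP_Customer in the level when play begins.
; It rolls one random seed, then builds each customer's ID from that seed, the customer's array index and the sum of its display name's character codes.
; It writes the ID into the customer's Generation struct and calls FillGeneration on that customer.
; A leftover debug print of enum-based random math is never run.
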(event `self.ReceiveBeginPlay`
  (set `self.Seed` (`KismetMathLibrary.RandomInteger` 650))
  (bind _outactors (`GameplayStatics.GetAllActorsOfClass` "/Game/Blueprints/AI_Thief/BP_Customer.BP_Customer_C"))
  (for (_array_element _array_index) _outactors
    (set `self.Temp` 0)
    (for _array_element_2 (`KismetStringLibrary.GetCharacterArrayFromString` (`KismetSystemLibrary.GetDisplayName` _array_element))
      (set `self.Temp` (+ (`self.Temp`) (`KismetStringLibrary.GetCharacterAsNumber` _array_element_2))))
    (bind _structout (setmembers `/Game/Blueprints/AI_Thief/STR_Generation` :`StructRef` (`/Game/Blueprints/AI_Thief/BP_Customer.Generation` _array_element) :`ID` (+ _array_index (`self.Seed`) (`self.Temp`))))
    (set `/Game/Blueprints/AI_Thief/BP_Customer.Generation` _structout _array_element)
    (`/Game/Blueprints/AI_Thief/BP_Customer.FillGeneration` _array_element)))

(event `self.ReceiveTick`
  (params (DeltaSeconds :type "Float (single-precision)")))

(fn `UserConstructionScript`)
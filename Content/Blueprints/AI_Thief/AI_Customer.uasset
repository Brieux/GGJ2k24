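; AI controller for shop customer NPCs, which starts their behavior tree and recycles them for repeat visits.
; After a random delay on BeginPlay, it caches the BP_Customer pawn, runs BT_Customer, begins shop navigation and resets the Behaviour blackboard key.
; CleanBeforeReplay clears the customer's state flags and type, then calls Replay, which waits a shorter random delay, restarts brain logic and re-enters the same startup sequence.
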(event `Replay`
  (`KismetSystemLibrary.Delay` (`KismetMathLibrary.RandomFloatInRange` 0.0 20.0))
  (`BrainComponent.RestartLogic` (`self.BrainComponent`))
  (bind _asbp_customer (cast `/Game/Blueprints/AI_Thief/BP_Customer` (`self.K2_GetPawn`) :!label _label))
  (set `self.BP_Customer` _asbp_customer)
  (`self.RunBehaviorTree` "/Game/Blueprints/AI_Thief/BT_Customer.BT_Customer")
  (`/Game/Blueprints/AI_Thief/BP_Customer.BeginNavigationInShop` _asbp_customer)
  (set `self.BlackBoardRef` (`AIBlueprintHelperLibrary.GetBlackboard` null))
  (`BlackboardComponent.SetValueAsEnum` (`self.BlackBoardRef`) "Behaviour" 0))

(event `self.ReceiveBeginPlay`
  (`KismetSystemLibrary.Delay` (`KismetMathLibrary.RandomFloatInRange` 20.0 65.0))
  (goto _label))

(event `CleanBeforeReplay`
  (bind _bp_customer (`self.BP_Customer`))
  (set `/Game/Blueprints/AI_Thief/BP_Customer.BuySomething ` false _bp_customer)
  (set `/Game/Blueprints/AI_Thief/BP_Customer.DecideToGetAway?` false _bp_customer)
  (set `/Game/Blueprints/AI_Thief/BP_Customer.hasBegunTask` false _bp_customer)
  (`/Game/Blueprints/AI_Thief/BP_Customer.SwitchType` _bp_customer false)
  (`self.Replay`))

(fn `UserConstructionScript`)
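; BP_Frigo is a fridge prop whose two glass panes break when hit.
; Each pane's first component hit adds a Geometry Collection component at that pane's relative transform, then destroys the original pane component.
; The same hit spawns a scaled-up FS_MasterField1 actor alongside the Geometry Collection.
; A separate DoOnce per pane limits each swap to a single trigger.
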(event `self.ReceiveBeginPlay`)

(event `self.S_FrigoVitre_A.OnComponentHit`
  (params (HitComponent :type "PrimitiveComponent Object Reference") (OtherActor :type "Actor Object Reference") (OtherComp :type "PrimitiveComponent Object Reference") (NormalImpulse :type "Vector Structure") (Hit :type "HitResult Structure (by ref)"))
  (`/Engine/EditorBlueprintResources/StandardMacros.DoOnce` false
    (:`Completed`
      (`AddComponent|NODE_AddGeometryCollectionComponent-0` :`RelativeTransform` (`SceneComponent.GetRelativeTransform` (`self.S_FrigoVitre_A`)))
      (`|SpawnActorFromClass` "/Game/FS_MasterField1.FS_MasterField1_C" (`KismetMathLibrary.MakeTransform` (0.0 0.0 0.0) (struct) (2.0 2.0 2.0)) "Undefined" "MultiplyWithRoot" null null)
      (`ActorComponent.K2_DestroyComponent` (`self.S_FrigoVitre_A`)))))

(event `self.S_FrigoVitre_A1.OnComponentHit`
  (params (HitComponent :type "PrimitiveComponent Object Reference") (OtherActor :type "Actor Object Reference") (OtherComp :type "PrimitiveComponent Object Reference") (NormalImpulse :type "Vector Structure") (Hit :type "HitResult Structure (by ref)"))
  (`/Engine/EditorBlueprintResources/StandardMacros.DoOnce` false
    (:`Completed`
      (`AddComponent|NODE_AddGeometryCollectionComponent-1` :`RelativeTransform` (`SceneComponent.GetRelativeTransform` (`self.S_FrigoVitre_A1`)))
      (`|SpawnActorFromClass` "/Game/FS_MasterField1.FS_MasterField1_C" (`KismetMathLibrary.MakeTransform` (0.0 0.0 0.0) (struct) (2.0 2.0 2.0)) "Undefined" "MultiplyWithRoot" null null)
      (`ActorComponent.K2_DestroyComponent` (`self.S_FrigoVitre_A1`)))))

(fn `UserConstructionScript`)
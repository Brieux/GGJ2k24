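; Product prop that takes a random mesh from a data table and can be grabbed as a physics object.
; Construction script and BeginPlay each use Index to choose a table row, then roll a random entry from its Product map; BeginPlay also enables physics a tick later.
; Grab resets rotation, locks the supplied constraint's angular motion, overrides mass, ignores PhysicsBody collisions and returns the mesh.
; The hit-triggered physics logic is disconnected.
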(event `self.ReceiveBeginPlay`
  (`KismetSystemLibrary.DelayUntilNextTick`)
  (`PrimitiveComponent.SetSimulatePhysics` (`self.StaticMesh`) true)
  (bind _outrownames (`DataTableFunctionLibrary.GetDataTableRowNames` (`self.Data Table`)))
  (bind _returnvalue (`|GetDataTableRow` (`self.Data Table`) (`|GetArrayItem` _outrownames (`KismetMathLibrary.FTrunc` (* (`self.index`) 10.0))))
    (:`then`
      (bind _product (break `/Game/Blueprints/Props/MiscProduct/Struct_Product` _returnvalue))
      (bind _keys (`BlueprintMapLibrary.Map_Keys` _product))
      (`StaticMeshComponent.SetStaticMesh` (`self.StaticMesh`) (`BlueprintMapLibrary.Map_Find` _product (`KismetArrayLibrary.Array_Random` _keys))))))

(event `self.StaticMesh.OnComponentHit`
  (params (HitComponent :type "PrimitiveComponent Object Reference") (OtherActor :type "Actor Object Reference") (OtherComp :type "PrimitiveComponent Object Reference") (NormalImpulse :type "Vector Structure") (Hit :type "HitResult Structure (by ref)")))

(fn `Grab`
  (params (PhysicsComp :type "PhysicsConstraintComponent Object Reference"))
  (returns (GrabbedComponent :type "PrimitiveComponent Object Reference"))
  (bind _staticmesh (`self.StaticMesh`))
  (`SceneComponent.K2_SetWorldRotation` :`self` (`self.StaticMesh`))
  (`PhysicsConstraintComponent.SetAngularSwing1Limit` PhysicsComp "ACM_Locked" 0.0)
  (`PhysicsConstraintComponent.SetAngularSwing2Limit` PhysicsComp "ACM_Locked" 0.0)
  (`PhysicsConstraintComponent.SetAngularTwistLimit` PhysicsComp "ACM_Locked" 0.0)
  (`PrimitiveComponent.SetSimulatePhysics` _staticmesh true)
  (`PrimitiveComponent.SetMassOverrideInKg` _staticmesh "None" 1.0 true)
  (`PrimitiveComponent.SetCollisionResponseToChannel` (`self.StaticMesh`) "ECC_PhysicsBody" "ECR_Ignore")
  (return (`self.StaticMesh`)))

(fn `UserConstructionScript`
  (bind _outrownames (`DataTableFunctionLibrary.GetDataTableRowNames` (`self.Data Table`)))
  (bind _returnvalue (`|GetDataTableRow` (`self.Data Table`) (`|GetArrayItem` _outrownames (`KismetMathLibrary.FTrunc` (* (`self.index`) 10.0))))
    (:`then`
      (bind _product (break `/Game/Blueprints/Props/MiscProduct/Struct_Product` _returnvalue))
      (bind _keys (`BlueprintMapLibrary.Map_Keys` _product))
      (`StaticMeshComponent.SetStaticMesh` (`self.StaticMesh`) (`BlueprintMapLibrary.Map_Find` _product (`KismetArrayLibrary.Array_Random` _keys))))))
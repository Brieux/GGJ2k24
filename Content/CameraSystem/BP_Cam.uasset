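; A grabbable TV camera system that cycles one scene capture through preset camera locations, rendering to a render target with a VHS post-process material.
; Construction applies the dynamic material and detaches the capture; BeginPlay starts a looping timer.
; SwitchCam's timeline animates the glitch parameter and, on its event track, moves the capture and updates the camera-index parameter.
; Grab locks the passed constraint's angular motion and returns the physics-simulated TV; Ungrab is empty.
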(event `self.ReceiveBeginPlay`
  (`KismetSystemLibrary.K2_SetTimerDelegate` (`|CreateDelegate` :!event `SwitchCam`) 1.0 true))

(event `SwitchCam`
  (bind (_output_location _output_rotation) (`KismetMathLibrary.BreakTransform` (`|GetArrayItem` (`self.CamLocations`) (`self.CurrentCam`))))
  (bind (_direction _bugvalue) (`Timeline|Timeline` :!via `PlayFromStart`)
    (:`Update`
      (`MaterialInstanceDynamic.SetScalarParameterValue` (`self.PostProMat`) "BUG" (* _bugvalue 10.0)))
    (:`EventSwitch`
      (bind _output_get (set `self.CurrentCam` (`KismetMathLibrary.Wrap` (+ (`self.CurrentCam`) 1) -1 (`KismetArrayLibrary.Array_LastIndex` (`self.CamLocations`)))))
      (`MaterialInstanceDynamic.SetScalarParameterValue` (`self.PostProMat`) "cam" (`KismetMathLibrary.Conv_IntToDouble` _output_get))
      (`SceneComponent.K2_SetWorldLocationAndRotation` (`self.SceneCaptureComponent2D`) _output_location _output_rotation false false))))

(fn `Grab`
  (params (PhysicsComp :type "PhysicsConstraintComponent Object Reference"))
  (returns (GrabbedComponent :type "PrimitiveComponent Object Reference"))
  (bind _tv (`self.TV`))
  (`PhysicsConstraintComponent.SetAngularSwing1Limit` PhysicsComp "ACM_Locked" 0.0)
  (`PhysicsConstraintComponent.SetAngularSwing2Limit` PhysicsComp "ACM_Locked" 0.0)
  (`PhysicsConstraintComponent.SetAngularTwistLimit` PhysicsComp "ACM_Locked" 0.0)
  (`PrimitiveComponent.SetSimulatePhysics` _tv true)
  (`PrimitiveComponent.SetMassOverrideInKg` _tv "None" 1.0 true)
  (`PrimitiveComponent.SetCollisionResponseToChannel` (`self.TV`) "ECC_PhysicsBody" "ECR_Ignore")
  (`PrimitiveComponent.SetCollisionResponseToChannel` (`self.TV`) "ECC_Pawn" "ECR_Ignore")
  (return (`self.TV`)))

(fn `Ungrab`
  (return))

(fn `UserConstructionScript`
  (bind _returnvalue (`KismetMaterialLibrary.CreateDynamicMaterialInstance` "/Game/PP/PP_VHS.PP_VHS"))
  (set `self.PostProMat` _returnvalue)
  (setmembers `PostProcessSettings` :`StructRef` (`SceneCaptureComponent2D.PostProcessSettings` (`self.SceneCaptureComponent2D`)) :`WeightedBlendables` (make `WeightedBlendables` (`|MakeArray` (make `WeightedBlendable` 1.0 (`self.PostProMat`)) :!type "WeightedBlendable Structure")))
  (set `SceneCaptureComponent2D.TextureTarget` (`self.TextureTarget`) (`self.SceneCaptureComponent2D`))
  (`SceneComponent.K2_DetachFromComponent` (`self.SceneCaptureComponent2D`) "KeepRelative" "KeepRelative" "KeepRelative" true))